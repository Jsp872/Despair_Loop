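; BP_RoomBase is the base combat room, locking the player in on bounds overlap and running a randomly selected set of enemy waves.
; Each wave spawns enemies at distinct random child spawn points, and EnemyDied counts them down to advance waves.
; Clearing the last wave disables exit blocker collision, increments the GameMode's cleared count, pauses, and offers three random upgrades filtered by selected ultimate.
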(event OnComponentBeginOverlap(RoomBounds)
  (params (OverlappedComponent :type Primitive%20Component%20Object%20Reference) (OtherActor :type Actor%20Object%20Reference) (OtherComp :type Primitive%20Component%20Object%20Reference) (OtherBodyIndex :type Integer) (bFromSweep :type Boolean) (SweepResult :type Hit%20Result%20Structure%20%28by%20ref%29))
  (Utilities|Casting|CastToBP_PlayerBase OtherActor)
  (if (not (Variables|Default|GetCombatStarted))
    (CallFunction|StartCombat)))

(event EventBeginPlay
  (for _array_element (Actor|GetAllChildActors true)
    (bind _asbp_enemy_spawn_point (Utilities|Casting|CastToBP_EnemySpawnPoint _array_element))
    (Utilities|Array|Add (Variables|Default|GetEnemiesSpawn) _asbp_enemy_spawn_point)
    (Variables|Default|SetWaveSelected (.waveset (.OutItem (Utilities|Array|Random (Variables|Default|GetWaveSet)))))))

(fn ConstructionScript)

(fn StartCombat
  (Variables|Default|SetCombatStarted true)
  (Collision|SetCollisionEnabled (Variables|Default|GetDoorBlockerEnter) "QueryAndPhysics")
  (CallFunction|StartWave))

(fn EnemyDied
  (bind _result (Math|Integer|DecrementInt (Variables|Default|GetAliveEnemies))
    (:%20%20
      (if (<= _result 0)
        (bind _result_2 (Math|Integer|IncrementInt (Variables|Default|GetCurrentWave))
          (:%20%20
            (if (>= (Variables|Default|GetCurrentWave) (Utilities|Array|Length (Variables|Default|GetWaveSelected)))
              (CallFunction|ClearRoom)
              (else
                (CallFunction|StartWave _result_2)))))))))

(fn ClearRoom
  (bind _returnvalue (Game|GetPlayerCharacter 0))
  (bind _asbp_player_base (Utilities|Casting|CastToBP_PlayerBase _returnvalue))
  (bind _availableupgrades (Variables|/Game/Blueprint/Player/BP_PlayerBase.BP_PlayerBase_C|GetAvailableUpgrades _asbp_player_base))
  (Variables|Default|SetRoomCleared true)
  (Collision|SetCollisionEnabled (Variables|Default|GetDoorBlockerExit) "NoCollision")
  (Math|Integer|IncrementInt (Variables|/Game/Blueprint/Core/BP_ThirdPersonGameMode.BP_ThirdPersonGameMode_C|GetClearedRooms (.AsBP%20Third%20Person%20Game%20Mode (Utilities|Casting|CastToBP_ThirdPersonGameMode (Game|GetGameMode))))
    (:%20%20
      (Game|SetGamePaused true)
      (while (< (Utilities|Array|Length (Variables|Default|GetRandomUpgrades)) 3)
        (bind _output_get (Variables|Default|SetUpgradeToCheck (Utilities|Array|Get(acopy) _availableupgrades (Math|Random|RandomIntegerinRange 0 (- (Utilities|Array|Length _availableupgrades) 1)))))
        (if (.IsUltimateSpecific (Utilities|Struct|BreakST_UpgradeData _output_get))
          (if (Utilities|Enum|Equal(Enum) (.RequiredUltimate (Utilities|Struct|BreakST_UpgradeData _output_get)) (Variables|/Game/Blueprint/Core/BP_GameInstance.BP_GameInstance_C|GetSelectedUltimate (.AsBP%20Game%20Instance (Utilities|Casting|CastToBP_GameInstance (Game|GetGameInstance)))))
            (Utilities|Array|Add (Variables|Default|GetRandomUpgrades) _output_get :!label _label))
          (else
            (goto _label))))
      (bind _returnvalue_2 (UserInterface|CreateWidget "/Game/UI/WBP_UpgradeChoice.WBP_UpgradeChoice_C" 0 (Variables|Default|GetRandomUpgrades)))
      (UserInterface|Viewport|AddtoViewport _returnvalue_2 0))))

(fn StartWave
  (params (WaveIndex :type Integer))
  (Variables|Default|SetAvailableSpawnPoints (Variables|Default|GetEnemiesSpawn))
  (for _array_element (.enemies (Utilities|Array|Get(acopy) (Variables|Default|GetWaveSelected) WaveIndex))
    (for _index (range 1 (.enemycount _array_element))
      (bind _output_get (Variables|Default|SetSelectedSpawnPoint (Utilities|Array|Get(acopy) (Variables|Default|GetAvailableSpawnPoints) (Math|Random|RandomInteger (Utilities|Array|Length (Variables|Default|GetAvailableSpawnPoints))))))
      (Utilities|Array|RemoveItem (Variables|Default|GetAvailableSpawnPoints) _output_get)
      (bind _returnvalue (Game|SpawnActorfromClass (.enemyclass _array_element) (Transformation|GetWorldTransform (Variables|/Game/Blueprint/Rooms/BP_EnemySpawnPoint.BP_EnemySpawnPoint_C|GetArrow _output_get)) "AlwaysSpawn" "MultiplyWithRoot" 0 0))
      (Variables|/Game/Blueprint/Enemy/BP_EnemyBase.BP_EnemyBase_C|SetOwnerRoom _returnvalue self)
      (Utilities|Array|Add (Variables|Default|GetSpawnedEnemies) _returnvalue)
      (Math|Integer|IncrementInt (Variables|Default|GetAliveEnemies)))))
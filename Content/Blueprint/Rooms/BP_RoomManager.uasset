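; BP_RoomManager builds a linear chain of rooms at BeginPlay, running from a spawn room through randomly chosen rooms to a boss room.
; Each room spawns at the ExitPoint transform of the previous one, so the layout chains end to end.
; Middle rooms are drawn from AllRoomsTypes with no duplicate check.
; SpawnedRooms records the classes of the spawn and middle rooms, but not the boss room.
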(event EventBeginPlay
  (bind _returnvalue (Game|SpawnActorfromClass "/Game/Blueprint/Rooms/BP_Room_Spawn.BP_Room_Spawn_C" (Math|Transform|MakeTransform "0.000000,0.000000,200.000000" "0, 0, 0" "1.000000,1.000000,1.000000") "Undefined" "MultiplyWithRoot" 0 0))
  (Variables|Default|SetNextRoomSpawn (Variables|/Game/Blueprint/Rooms/BP_RoomBase.BP_RoomBase_C|GetExitPoint _returnvalue))
  (Utilities|Array|Add (Variables|Default|GetSpawnedRooms) (Utilities|GetClass _returnvalue))
  (for _index (range 0 3)
    (bind _returnvalue_2 (Game|SpawnActorfromClass (.OutItem (Utilities|Array|Random (Variables|Default|GetAllRoomsTypes))) (Transformation|GetWorldTransform (Variables|Default|GetNextRoomSpawn)) "Undefined" "MultiplyWithRoot" 0 0))
    (Variables|Default|SetNextRoomSpawn (Variables|/Game/Blueprint/Rooms/BP_RoomBase.BP_RoomBase_C|GetExitPoint _returnvalue_2))
    (Utilities|Array|Add (Variables|Default|GetSpawnedRooms) (Utilities|GetClass _returnvalue_2)))
  (Game|SpawnActorfromClass "/Game/Blueprint/Rooms/BP_Room_Boss.BP_Room_Boss_C" (Transformation|GetWorldTransform (Variables|Default|GetNextRoomSpawn)) "Undefined" "MultiplyWithRoot" 0 0))

(fn ConstructionScript)
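; Upgrade Blueprint that raises the player's critical hit chance.
; It overrides ApplyUpgrade to add CritChanceToAdd to the player's CritChance, clamped to a 0–100 range, then calls the parent implementation.
; The event graph holds only disabled default events, so all of its own logic lives in that override.
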(event EventBeginPlay
  (|CallParentFunction) ; This node is disabled and will not be called.\nDrag off pins to build functionality.
)

(event Collision|EventActorBeginOverlap
  (params (OtherActor :type Actor%20Object%20Reference))
  (|CallParentFunction OtherActor) ; This node is disabled and will not be called.\nDrag off pins to build functionality.
)

(event EventTick
  (params (DeltaSeconds :type Float%20%28single-precision%29))
  (|CallParentFunction DeltaSeconds) ; This node is disabled and will not be called.\nDrag off pins to build functionality.
)

(fn ConstructionScript
  (|CallParentFunction))

(fn ApplyUpgrade
  (params (PlayerReference :type BP%20Player%20Base%20Object%20Reference))
  (Variables|/Game/Blueprint/Player/BP_PlayerBase.BP_PlayerBase_C|SetCritChance PlayerReference (Math|Float|Clamp(Float) (+ (Variables|/Game/Blueprint/Player/BP_PlayerBase.BP_PlayerBase_C|GetCritChance PlayerReference) (Variables|Default|GetCritChanceToAdd)) 0.0 1e+02))
  (|CallParentFunction PlayerReference))
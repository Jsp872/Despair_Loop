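; Boss enemy Blueprint for Monokuma that picks one of two attacks at random on a looping timer started at BeginPlay.
; One attack is a short dash: it temporarily raises the character's max walk speed, then lowers it after a delay.
; The other turns the boss in yaw to face the first player and spawns a damaging projectile at its ProjectileSpawn point.
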(event Custom|Attack
  (if (== (Math|Random|RandomInteger 2) 0)
    (Variables|/Script/Engine.CharacterMovementComponent|SetMaxWalkSpeed (Variables|Character|GetCharacterMovement) 7e+02)
    (Utilities|FlowControl|Delay 2.0)
    (Variables|/Script/Engine.CharacterMovementComponent|SetMaxWalkSpeed (Variables|Character|GetCharacterMovement) 2e+02)
    (else
      (Transformation|SetActorRotation (Math|Rotator|MakeRotator 0.0 0.0 (.Yaw (Math|Rotator|BreakRotator (Math|Rotator|FindLookatRotation (Transformation|GetActorLocation) (Transformation|GetActorLocation (Game|GetPlayerCharacter 0)))))))
      (Game|SpawnActorfromClass (Variables|Default|GetProjectileClass) (Transformation|GetWorldTransform (Variables|Default|GetProjectileSpawn)) "Undefined" "MultiplyWithRoot" 0 5.0 "NewEnumerator1" false 0))))

(event EventBeginPlay
  (|CallParentFunction)
  (Utilities|Time|SetTimerbyEvent (delegate Custom|Attack) 3.0 true))

(fn ConstructionScript
  (|CallParentFunction))
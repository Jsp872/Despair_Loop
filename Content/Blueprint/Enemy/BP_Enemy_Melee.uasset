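; Melee enemy Blueprint that chases the player and deals repeated damage at close range.
; A looping timer started on BeginPlay reissues AI MoveTo toward the player character.
; DamageZone overlap with a BP_PlayerBase starts a looping attack timer, which applies Damage while CanAttack is true and the player is valid.
; Any actor ending overlap with DamageZone clears that timer, without checking that it is the player.
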(event OnComponentBeginOverlap(DamageZone)
  (params (OverlappedComponent :type Primitive%20Component%20Object%20Reference) (OtherActor :type Actor%20Object%20Reference) (OtherComp :type Primitive%20Component%20Object%20Reference) (OtherBodyIndex :type Integer) (bFromSweep :type Boolean) (SweepResult :type Hit%20Result%20Structure%20%28by%20ref%29))
  (bind _asbp_player_base (Utilities|Casting|CastToBP_PlayerBase OtherActor))
  (bind _returnvalue (Utilities|Time|SetTimerbyEvent (delegate Custom|AttackPlayer) 1.0 true))
  (Variables|Default|SetAttackCooldown _returnvalue))

(event OnComponentEndOverlap(DamageZone)
  (params (OverlappedComponent :type Primitive%20Component%20Object%20Reference) (OtherActor :type Actor%20Object%20Reference) (OtherComp :type Primitive%20Component%20Object%20Reference) (OtherBodyIndex :type Integer))
  (Utilities|Time|ClearandInvalidateTimerbyHandle (Variables|Default|GetAttackCooldown)))

(event Custom|AttackPlayer
  (if (Variables|Default|GetCanAttack)
    (Utilities|IsValid (stale OnComponentBeginOverlap(DamageZone) _asbp_player_base)
      (:Is%20Valid
        (Default|TakeDamage (stale OnComponentBeginOverlap(DamageZone) _asbp_player_base) (Variables|Default|GetDamage))))))

(event Custom|FollowPlayer
  (AI|AIMoveTo self "0, 0, 0" (Game|GetPlayerCharacter 0) 1.2e+02 false))

(event EventBeginPlay
  (|CallParentFunction)
  (Utilities|Time|SetTimerbyEvent (delegate Custom|FollowPlayer) 0.2 true))

(fn ConstructionScript
  (|CallParentFunction))
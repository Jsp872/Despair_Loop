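; Kamikaze enemy that starts a timed self-destruct when a player enters its damage zone.
; Triggering zeroes its walk speed and runs two timers: a looping orange flash with scale pulse, and the delayed explosion.
; The blast spawns a Niagara effect and uses a sphere overlap to damage both players and other enemies.
; It then kills itself by applying massive damage through TakeDamage.
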(event OnComponentBeginOverlap(DamageZone)
  (params (OverlappedComponent :type Primitive%20Component%20Object%20Reference) (OtherActor :type Actor%20Object%20Reference) (OtherComp :type Primitive%20Component%20Object%20Reference) (OtherBodyIndex :type Integer) (bFromSweep :type Boolean) (SweepResult :type Hit%20Result%20Structure%20%28by%20ref%29))
  (Utilities|Casting|CastToBP_PlayerBase OtherActor)
  (if (not (Variables|Default|GetIsExploding))
    (CallFunction|StartExplosion)))

(event Custom|StartExplosion
  (Variables|Default|SetIsExploding true)
  (Variables|/Script/Engine.CharacterMovementComponent|SetMaxWalkSpeed (Variables|Character|GetCharacterMovement) 0.0)
  (Utilities|Time|SetTimerbyEvent (delegate Custom|StartExplosionAnim) 0.2 true)
  (Utilities|Time|SetTimerbyEvent (delegate Custom|Explose) (Variables|Default|GetExplosionDelay)))

(event Custom|StartExplosionAnim
  (bind _mesh (Variables|Character|GetMesh))
  (CallFunction|Flash "1.000000,0.300000,0.000000" 0.1)
  (Transformation|SetWorldScale3D _mesh "1.200000,1.200000,1.200000")
  (Utilities|FlowControl|Delay 0.1)
  (Transformation|SetWorldScale3D _mesh "1.000000,1.000000,1.000000"))

(event Custom|Explose
  (bind _returnvalue (Transformation|GetActorTransform))
  (Niagara|SpawnSystematLocation "/Game/FX/VFX/NS_KamikazeExplosion.NS_KamikazeExplosion" (.location _returnvalue) (.rotation _returnvalue))
  (bind _outactors (Collision|SphereOverlapActors (Transformation|GetWorldLocation (Variables|Character|GetMesh)) (Variables|Default|GetExplosionRadius) (Variables|Default|GetObject%20Types) 0))
  (for _array_element _outactors
    (bind _asbp_player_base (Utilities|Casting|CastToBP_PlayerBase _array_element)
      (:then
        (Default|TakeDamage _asbp_player_base (Variables|Default|GetExplosionDamage)))
      (:CastFailed
        (bind _asbp_enemy_base (Utilities|Casting|CastToBP_EnemyBase _array_element))
        (Default|TakeDamage _asbp_enemy_base (Variables|Default|GetExplosionDamage) false))))
  (CallFunction|TakeDamage 55555.0 false))

(event EventBeginPlay
  (|CallParentFunction) ; This node is disabled and will not be called.\nDrag off pins to build functionality.
)

(event Collision|EventActorBeginOverlap
  (params (OtherActor :type Actor%20Object%20Reference))
  (|CallParentFunction OtherActor) ; This node is disabled and will not be called.\nDrag off pins to build functionality.
)

(event EventTick
  (params (DeltaSeconds :type Float%20%28single-precision%29))
  (|CallParentFunction DeltaSeconds) ; This node is disabled and will not be called.\nDrag off pins to build functionality.
)

(fn ConstructionScript
  (|CallParentFunction))
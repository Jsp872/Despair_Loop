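; Ranged enemy Blueprint that periodically fires projectiles at the first player's character.
; After the parent's BeginPlay, a looping timer set to Cooldown calls ShootProjectile, which acts only while CanAttack is true.
; Each shot snaps the enemy's yaw toward the player, then spawns ProjectileClass at the actor's transform with fixed damage and an owner type.
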(event Custom|ShootProjectile
  (if (Variables|Default|GetCanAttack)
    (Transformation|SetActorRotation (Math|Rotator|MakeRotator 0.0 0.0 (.Yaw (Math|Rotator|BreakRotator (Math|Rotator|FindLookatRotation (Transformation|GetActorLocation) (Transformation|GetActorLocation (Game|GetPlayerCharacter 0)))))))
    (Game|SpawnActorfromClass (Variables|Default|GetProjectileClass) (Transformation|GetActorTransform) "Undefined" "MultiplyWithRoot" 0 5.0 "NewEnumerator1" false 0)))

(event EventBeginPlay
  (|CallParentFunction)
  (Utilities|Time|SetTimerbyEvent (delegate Custom|ShootProjectile) (Variables|Default|GetCooldown) true))

(fn ConstructionScript
  (|CallParentFunction))
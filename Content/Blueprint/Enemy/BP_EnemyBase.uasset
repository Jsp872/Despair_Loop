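; Base enemy character that handles damage, status effects and death, with brief invincibility after spawning.
; TakeDamage shows floating numbers, flashes the mesh via a HitColor material parameter, and can start stacking poison that ticks on a looping timer.
; ApplyHack temporarily slows movement and blocks attacks.
; Death awards random currency, notifies the owner room or shows victory for the final boss, applies player lifesteal, and plays a scale timeline before destruction.
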(event Custom|Flash
  (params (NewColor :type Vector) (DelayBetweenChange :type Float%20%28double-precision%29))
  (Rendering|Material|SetVectorParameterValueonMaterials (Variables|Character|GetMesh) "HitColor" NewColor)
  (Utilities|FlowControl|Delay DelayBetweenChange)
  (Rendering|Material|SetVectorParameterValueonMaterials (Variables|Character|GetMesh) "HitColor" "1.000000,1.000000,1.000000"))

(event Custom|CheckIfPoisoned
  (Variables|Default|SetPoisonCharge (+ (Variables|Default|GetPoisonCharge) 5))
  (if (not (Variables|Default|GetPoisoned))
    (Variables|Default|SetPoisoned true)
    (bind _returnvalue (Utilities|Time|SetTimerbyEvent (delegate Custom|ApplyPoison) 1.0 true))
    (Variables|Default|SetPoisonCooldown _returnvalue)))

(event Custom|ApplyPoison
  (if (> (Variables|Default|GetPoisonCharge) 0)
    (CallFunction|TakeDamage 5.0 false)
    (Math|Integer|DecrementInt (Variables|Default|GetPoisonCharge))
    (else
      (Utilities|Time|ClearandInvalidateTimerbyHandle (Variables|Default|GetPoisonCooldown))
      (Variables|Default|SetPoisoned false))))

(event Custom|Invincibility
  (Variables|Default|SetisInvincible false))

(event Custom|DeathAnimation
  (bind _returnvalue (Transformation|GetActorTransform))
  (Niagara|SpawnSystematLocation "/Game/FX/VFX/NS_EnemyDeath.NS_EnemyDeath" (.location _returnvalue) (.rotation _returnvalue) (.scale _returnvalue))
  (AI|Navigation|StopMovement (Pawn|GetController))
  (Pawn|Components|CharacterMovement|DisableMovement (Variables|Character|GetCharacterMovement))
  (Collision|SetCollisionEnabled (Variables|Collision|GetCapsuleComponent) "NoCollision")
  (bind _newtrack_0 (Timeline|TL_Death Play)
    (:Update
      (Transformation|SetWorldScale3D (Variables|Character|GetMesh) (Math|Conversions|ToVector(Float) _newtrack_0)))
    (:Finished
      (Actor|DestroyActor))))

(event Custom|ApplyHack
  (params (SlowMultiplier :type Float%20%28double-precision%29) (Duration :type Float%20%28double-precision%29))
  (Variables|/Script/Engine.CharacterMovementComponent|SetMaxWalkSpeed (Variables|Character|GetCharacterMovement) (* SlowMultiplier (Variables|Default|GetDefaultMoveSpeed)))
  (Utilities|Time|SetTimerbyEvent (delegate Custom|ResetSlow) Duration)
  (Variables|Default|SetCanAttack false)
  (Utilities|Time|SetTimerbyEvent (delegate Custom|StunAttack) 1.0))

(event Custom|ResetSlow
  (Variables|/Script/Engine.CharacterMovementComponent|SetMaxWalkSpeed (Variables|Character|GetCharacterMovement) (Variables|Default|GetDefaultMoveSpeed)))

(event Custom|StunAttack
  (Variables|Default|SetCanAttack true))

(event EventBeginPlay
  (bind _returnvalue (Rendering|Material|CreateDynamicMaterialInstance (Variables|Character|GetMesh) 0 0 "None" :!class /Script/Engine.PrimitiveComponent))
  (Variables|Default|SetDynamicMaterial _returnvalue)
  (Utilities|Time|SetTimerbyEvent (delegate Custom|Invincibility) 0.2)
  (Variables|/Script/Engine.CharacterMovementComponent|SetMaxWalkSpeed (Variables|Character|GetCharacterMovement) (Variables|Default|GetDefaultMoveSpeed)))

(fn ConstructionScript)

(fn TakeDamage
  (params (DamageAmount :type Float%20%28double-precision%29) (HasPoison :type Boolean))
  (bind _returnvalue (Game|GetPlayerCharacter 0))
  (bind _returnvalue_2 (Game|GetGameInstance))
  (bind _asbp_game_instance (Utilities|Casting|CastToBP_GameInstance _returnvalue_2))
  (bind _asbp_player_base (Utilities|Casting|CastToBP_PlayerBase _returnvalue))
  (bind _lifesteal (Variables|/Game/Blueprint/Player/BP_PlayerBase.BP_PlayerBase_C|GetLifesteal _asbp_player_base))
  (if (not (Variables|Default|GetisInvincible))
    (Game|SpawnActorfromClass "/Game/Blueprint/BP_FloatingDamage.BP_FloatingDamage_C" (Math|Conversions|ToTransform(Vector) (+ (Transformation|GetActorLocation) (Math|Vector|MakeVector (Math|Random|RandomFloatinRange -3e+01 3e+01) (Math|Random|RandomFloatinRange -3e+01 3e+01) 1e+02))) "Undefined" "MultiplyWithRoot" 0 DamageAmount 0)
    (UserInterface|CreateWidget "/Game/UI/WBP_FloatingDamage.WBP_FloatingDamage_C" 0 (Utilities|Text|ToText(Float) DamageAmount "HalfToEven"))
    (if HasPoison
      (CallFunction|CheckifPoisoned))
    (bind _output_get (Variables|Default|SetCurrentHealth (- (Variables|Default|GetCurrentHealth) DamageAmount)))
    (CallFunction|Flash "3.000000,0.000000,0.000000" 0.2)
    (if (<= _output_get 0.0)
      (if (not (Variables|Default|GetIsDead))
        (Variables|Default|SetIsDead true)
        (Variables|/Game/Blueprint/Core/BP_GameInstance.BP_GameInstance_C|SetMonopieces _asbp_game_instance (+ (Variables|/Game/Blueprint/Core/BP_GameInstance.BP_GameInstance_C|GetMonopieces _asbp_game_instance) (Math|Random|RandomIntegerinRange (Variables|Default|GetMinMonocoinsGiveAtDeath) (Variables|Default|GetMaxMonocoinsGiveAtDeath))))
        (Default|UpdateHUD (Variables|/Game/Blueprint/Core/BP_ThirdPersonPlayerController.BP_ThirdPersonPlayerController_C|GetHUDReference (.AsBP%20Third%20Person%20Player%20Controller (Utilities|Casting|CastToBP_ThirdPersonPlayerController (Game|GetPlayerController 0)))))
        (if (Variables|Default|GetisFinalBoss)
          (bind _returnvalue_3 (UserInterface|CreateWidget "/Game/UI/WBP_Victory.WBP_Victory_C"))
          (UserInterface|Viewport|AddtoViewport _returnvalue_3 0)
          (else
            (Default|EnemyDied (Variables|Default|GetOwnerRoom))))
        (CallFunction|DeathAnimation)
        (if (> _lifesteal 0.0)
          (Variables|/Game/Blueprint/Player/BP_PlayerBase.BP_PlayerBase_C|SetCurrentHealth _asbp_player_base (Math|Float|Clamp(Float) (+ _lifesteal (Variables|/Game/Blueprint/Player/BP_PlayerBase.BP_PlayerBase_C|GetCurrentHealth _asbp_player_base)) 0.0 (Variables|/Game/Blueprint/Player/BP_PlayerBase.BP_PlayerBase_C|GetMaxHealth _asbp_player_base))))))))
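; BP_PlayerRanged is a ranged player Blueprint whose normal and heavy attacks fire projectiles.
; Attack and HeavyAttack each pass their own projectile class to a shared ShootProjectile function.
; ShootProjectile spawns that projectile slightly ahead of the AttackSpawn component, facing the actor's rotation, with the player as owner and its damage and poison flag passed in.
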(event EventBeginPlay
  (|CallParentFunction) ; This node is disabled and will not be called.\nDrag off pins to build functionality.
)

(event Collision|EventActorBeginOverlap
  (params (OtherActor :type Actor%20Object%20Reference)))

(event EventTick
  (params (DeltaSeconds :type Float%20%28single-precision%29))
  (|CallParentFunction DeltaSeconds) ; This node is disabled and will not be called.\nDrag off pins to build functionality.
)

(fn ConstructionScript
  (|CallParentFunction))

(fn Attack
  (CallFunction|ShootProjectile (Variables|Default|GetNormalAttackProjectile)))

(fn HeavyAttack
  (CallFunction|ShootProjectile (Variables|Default|GetHeavyAttackProjectile)))

(fn ShootProjectile
  (params (ProjectileType :type BP%20Projectile%20Base%20Class%20Reference))
  (Game|SpawnActorfromClass ProjectileType (Math|Transform|MakeTransform (+ (Transformation|GetWorldLocation (Variables|Default|GetAttackSpawn)) (* (Transformation|GetActorForwardVector) 1e+02)) (Transformation|GetActorRotation) "1.000000,1.000000,1.000000") "Undefined" "MultiplyWithRoot" self (Variables|Default|GetDamageToDo) "NewEnumerator0" (Variables|Default|GetPoisonEnabled) 0))
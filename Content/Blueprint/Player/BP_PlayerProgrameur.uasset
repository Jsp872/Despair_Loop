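; Programmer player character, a child class that overrides shooting and three abilities with a hacking theme.
; Shooting spawns two side-by-side projectiles carrying damage and poison settings when double projectiles is on, otherwise defers to the parent.
; Its capacities drop a hack zone at its feet and spawn an owned drone.
; The ultimate plays a wave effect, briefly slows global time, then damages, hack-slows and marks every enemy found through GetAllActorsOfClass.
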(event Custom|FreezeTime
  (Utilities|Time|SetGlobalTimeDilation 0.2)
  (Utilities|FlowControl|Delay 0.15)
  (Utilities|Time|SetGlobalTimeDilation 1.0))

(event EventBeginPlay
  (|CallParentFunction))

(event EventTick
  (params (DeltaSeconds :type Float%20%28single-precision%29))
  (|CallParentFunction DeltaSeconds))

(fn ConstructionScript
  (|CallParentFunction))

(fn ShootProjectile
  (params (ProjectileType :type BP%20Projectile%20Base%20Class%20Reference))
  (bind _attackspawn (Variables|Default|GetAttackSpawn))
  (bind _attackspawn_2 (Variables|Default|GetAttackSpawn))
  (LocalVariables|SetProjectile ProjectileType)
  (if (Variables|Default|GetDoubleProjectiles)
    (Game|SpawnActorfromClass (LocalVariables|GetProjectile) (Math|Transform|MakeTransform (+ (* (Math|Vector|GetRightVector _attackspawn_2) 5e+01) (+ (Transformation|GetWorldLocation _attackspawn_2) (* (Transformation|GetActorForwardVector) 1e+02))) (Transformation|GetActorRotation) "1.000000,1.000000,1.000000") "Undefined" "MultiplyWithRoot" self (Variables|Default|GetDamageToDo) "NewEnumerator0" (Variables|Default|GetPoisonEnabled) 0)
    (Game|SpawnActorfromClass (LocalVariables|GetProjectile) (Math|Transform|MakeTransform (- (+ (Transformation|GetWorldLocation _attackspawn) (* (Transformation|GetActorForwardVector) 1e+02)) (* (Math|Vector|GetRightVector _attackspawn) 5e+01)) (Transformation|GetActorRotation) "1.000000,1.000000,1.000000") "Undefined" "MultiplyWithRoot" self (Variables|Default|GetDamageToDo) "NewEnumerator0" (Variables|Default|GetPoisonEnabled) 0)
    (else
      (|CallParentFunction ProjectileType))))

(fn Capacity1
  (bind _returnvalue (Transformation|GetActorTransform))
  (Game|SpawnActorfromClass "/Game/Blueprint/Weapons/BP_HackZone.BP_HackZone_C" (Math|Transform|MakeTransform (- (.location _returnvalue) "0.000000,0.000000,75.000000") (.rotation _returnvalue) (.scale _returnvalue)) "Undefined" "MultiplyWithRoot" 0 0))

(fn Capacity2
  (Game|SpawnActorfromClass "/Game/Blueprint/Weapons/BP_ProgrammerDrone.BP_ProgrammerDrone_C" (Transformation|GetActorTransform) "Undefined" "MultiplyWithRoot" 0 self 0))

(fn Ultimate
  (bind _returnvalue (Transformation|GetActorTransform))
  (Niagara|SpawnSystematLocation "/Game/FX/VFX/NS_HackWave.NS_HackWave" (.location _returnvalue) (.rotation _returnvalue) "10.000000,10.000000,10.000000")
  (CallFunction|FreezeTime)
  (bind _outactors (Actor|GetAllActorsOfClass "/Game/Blueprint/Enemy/BP_EnemyBase.BP_EnemyBase_C"))
  (for _array_element _outactors
    (Default|TakeDamage _array_element 99.0 (Variables|Default|GetPoisonEnabled))
    (Default|ApplyHack _array_element 0.3 5.0)
    (Niagara|SpawnSystemAttached "/Game/FX/VFX/NS_HackEnemy.NS_HackEnemy" (Variables|/Script/Engine.Character|GetMesh _array_element) "None" "0, 0, 0" "0, 0, 0" "KeepRelativeOffset" false)))
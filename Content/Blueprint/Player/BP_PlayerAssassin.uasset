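; Assassin player character that overrides the parent's attacks, two capacities and ultimate.
; Heavy attack is an invincible launch through pawns, damaging each enemy once via a toggled overlap zone; dash input can add an area hit.
; Capacity 1 grants timed invincibility, speed and a ghost material; Capacity 2 empowers the next normal or heavy attack.
; The ultimate is a timed berserk that scales move speed and attack and dash cooldowns from cached base values.
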(event OnComponentBeginOverlap(DashDamageZone)
  (params (OverlappedComponent :type Primitive%20Component%20Object%20Reference) (OtherActor :type Actor%20Object%20Reference) (OtherComp :type Primitive%20Component%20Object%20Reference) (OtherBodyIndex :type Integer) (bFromSweep :type Boolean) (SweepResult :type Hit%20Result%20Structure%20%28by%20ref%29))
  (if (Variables|Default|GetIsHeavyDashing)
    (bind _asbp_enemy_base (Utilities|Casting|CastToBP_EnemyBase OtherActor))
    (if (not (Utilities|Array|ContainsItem (Variables|Default|GetDamagedEnemies) _asbp_enemy_base))
      (Default|TakeDamage _asbp_enemy_base (Variables|Default|GetDamageToDo) (Variables|Default|GetPoisonEnabled))
      (Utilities|Array|Add (Variables|Default|GetDamagedEnemies) _asbp_enemy_base))))

(event Custom|EndHeavyAttack
  (Utilities|FlowControl|Delay (Variables|Default|GetHeavyDashDuration))
  (Variables|Default|SetIsHeavyDashing false)
  (Variables|Default|SetIsInvincible false)
  (Collision|SetCollisionEnabled (Variables|Default|GetDashDamageZone) "NoCollision")
  (Input|EnableInput 0)
  (Collision|SetCollisionResponsetoChannel (Variables|Default|GetCapsuleComponent) "ECC_Pawn" "ECR_Block"))

(event Custom|DoCapacity1
  (bind _charactermovement (Variables|Character|GetCharacterMovement))
  (bind _mesh (Variables|Character|GetMesh))
  (Niagara|SpawnSystematLocation "/Game/FX/VFX/NS_SmokeEscape.NS_SmokeEscape" (Transformation|GetActorLocation))
  (Niagara|SpawnSystemAttached "/Game/FX/VFX/NS_AssassinCapacity1Trail.NS_AssassinCapacity1Trail" (Variables|Character|GetMesh) "None" "0, 0, 0" "0, 0, 0" "KeepRelativeOffset" false)
  (Variables|/Script/Engine.CharacterMovementComponent|SetMaxWalkSpeed _charactermovement (* (Variables|/Script/Engine.CharacterMovementComponent|GetMaxWalkSpeed _charactermovement) 1.3))
  (Variables|Default|SetIsInvincible true)
  (Utilities|Time|SetTimerbyEvent (delegate Custom|ResetCapacity1) (Variables|Default|GetCapacity1Duration))
  (for (_ _array_index) (Rendering|Material|GetMaterials _mesh)
    (Rendering|Material|SetMaterial _mesh _array_index "/Game/Materials/M_Ghost.M_Ghost")))

(event Custom|ResetCapacity1
  (Variables|Default|SetIsInvincible false)
  (Variables|/Script/Engine.CharacterMovementComponent|SetMaxWalkSpeed (Variables|Character|GetCharacterMovement) (Variables|Default|GetMoveSpeed))
  (for (_array_element _array_index) (Variables|Default|GetOriginalMaterials)
    (Rendering|Material|SetMaterial (Variables|Character|GetMesh) _array_index _array_element)))

(event Custom|UseUltimate
  (Variables|/Script/Engine.CharacterMovementComponent|SetMaxWalkSpeed (Variables|Character|GetCharacterMovement) (* (Variables|Default|GetBerserkMoveMultiplier) (Variables|Default|GetMoveSpeed)))
  (Variables|Default|SetNormalAttackCooldown (* (Variables|Default|GetBaseAttackCooldown) (Variables|Default|GetBerserkAttackSpeedMultiplier)))
  (Variables|Default|SetDashCooldown (* (Variables|Default|GetBaseDashCooldown) (Variables|Default|GetBerserkDashCooldownMultiplier)))
  (bind _returnvalue (Niagara|SpawnSystemAttached "/Game/FX/VFX/NS_BerserkAura.NS_BerserkAura" (Variables|Character|GetMesh) "None" "0.000000,0.000000,100.000000" "0, 0, 0" "KeepRelativeOffset" false))
  (Variables|Default|SetBerserkAuraRef _returnvalue)
  (Utilities|Time|SetTimerbyEvent (delegate Custom|ResetStats) (Variables|Default|GetBerserkDuration)))

(event Custom|ResetStats
  (Variables|/Script/Engine.CharacterMovementComponent|SetMaxWalkSpeed (Variables|Character|GetCharacterMovement) (Variables|Default|GetMoveSpeed))
  (Variables|Default|SetNormalAttackCooldown (Variables|Default|GetBaseAttackCooldown))
  (Variables|Default|SetDashCooldown (Variables|Default|GetBaseDashCooldown))
  (Components|DestroyComponent (Variables|Default|GetBerserkAuraRef)))

(event Input|EnhancedActionEvents|EnhancedInputActionIA_Dash
  (params (ActionValue :type Boolean) (ElapsedSeconds :type Float%20%28double-precision%29) (TriggeredSeconds :type Float%20%28double-precision%29) (InputAction :type Input%20Action%20Object%20Reference :default "/Game/Input/Actions/IA_Dash.IA_Dash"))
  (:Started
    (if (Variables|Default|GetCanDash)
      (if (Variables|Default|GetDashDamageEnabled)
        (CallFunction|SetDamage (Variables|Default|GetAttackDamage))
        (bind _outactors (Collision|SphereOverlapActors (Transformation|GetWorldLocation (Variables|Default|GetCapsuleComponent)) 2.5e+02 (Variables|Default|GetObjectTypesToAttack) 0))
        (for _array_element _outactors
          (bind _asbp_enemy_base (Utilities|Casting|CastToBP_EnemyBase _array_element))
          (Default|TakeDamage _asbp_enemy_base (* (Variables|Default|GetDamageToDo) 2.0) (Variables|Default|GetPoisonEnabled)))))))

(event EventBeginPlay
  (|CallParentFunction)
  (Collision|SetCollisionEnabled (Variables|Default|GetDashDamageZone) "NoCollision")
  (for _array_element (Rendering|Material|GetMaterials (Variables|Character|GetMesh))
    (Utilities|Array|Add (Variables|Default|GetOriginalMaterials) _array_element)
    (Variables|Default|SetBaseAttackCooldown (Variables|Default|GetNormalAttackCooldown))
    (Variables|Default|SetBaseDashCooldown (Variables|Default|GetDashCooldown))))

(event Collision|EventActorBeginOverlap
  (params (OtherActor :type Actor%20Object%20Reference))
  (|CallParentFunction OtherActor) ; This node is disabled and will not be called.\nDrag off pins to build functionality.
)

(event EventTick
  (params (DeltaSeconds :type Float%20%28single-precision%29))
  (|CallParentFunction DeltaSeconds) ; This node is disabled and will not be called.\nDrag off pins to build functionality.
)

(fn ConstructionScript
  (|CallParentFunction))

(fn HeavyAttack
  (if (Variables|Default|GetHasEmpoweredAttack)
    (Variables|Default|SetDamageToDo (* (Variables|Default|GetDamageToDo) (Variables|Default|GetEmpowerMultiplier)))
    (Variables|Default|SetHasEmpoweredAttack false)
    (Components|DestroyComponent (Variables|Default|GetEmpoweredAuraRef)))
  (Input|DisableInput 0)
  (Character|LaunchCharacter (* (* (Variables|Default|GetDashDistance) 2.0) (Math|Vector|Normalize (Class|Pawn|GetLastMovementInputVector))) true false)
  (Variables|Default|SetIsHeavyDashing true)
  (Variables|Default|SetIsInvincible true)
  (Utilities|Array|Clear (Variables|Default|GetDamagedEnemies))
  (Collision|SetCollisionEnabled (Variables|Default|GetDashDamageZone) "QueryOnly")
  (Collision|SetCollisionResponsetoChannel (Variables|Default|GetCapsuleComponent) "ECC_Pawn" "ECR_Ignore")
  (Niagara|SpawnSystemAttached "/Game/FX/VFX/NS_AssassinDashTrail.NS_AssassinDashTrail" (Variables|Character|GetMesh) "None" "0, 0, 0" "0, 0, 0" "KeepRelativeOffset" false)
  (CallFunction|EndHeavyAttack))

(fn Capacity1
  (CallFunction|DoCapacity1))

(fn Capacity2
  (Variables|Default|SetHasEmpoweredAttack true)
  (bind _returnvalue (Niagara|SpawnSystemAttached "/Game/FX/VFX/NS_EmporedAura.NS_EmporedAura" (Variables|Character|GetMesh) "None" "0.000000,0.000000,50.000000" "0, 0, 0" "KeepRelativeOffset" false))
  (Variables|Default|SetEmpoweredAuraRef _returnvalue))

(fn Attack
  (if (Variables|Default|GetHasEmpoweredAttack)
    (Variables|Default|SetDamageToDo (* (Variables|Default|GetDamageToDo) (Variables|Default|GetEmpowerMultiplier)))
    (Variables|Default|SetHasEmpoweredAttack false)
    (Components|DestroyComponent (Variables|Default|GetEmpoweredAuraRef)))
  (|CallParentFunction))

(fn Ultimate
  (CallFunction|UseUltimate))
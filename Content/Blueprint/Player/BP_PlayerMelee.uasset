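; BP_PlayerMelee is a melee player Blueprint that deals area damage to enemies.
; Attack spawns a Niagara slash effect on the AttackSpawn component and runs a sphere overlap there, using a configurable radius and object types.
; Each overlapped BP_EnemyBase takes damage along with a flag for whether poison applies.
; BeginPlay, Tick and construction only call the parent class.
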(event EventBeginPlay
  (|CallParentFunction))

(event EventTick
  (params (DeltaSeconds :type Float%20%28single-precision%29))
  (|CallParentFunction DeltaSeconds))

(fn ConstructionScript
  (|CallParentFunction))

(fn Attack
  (Niagara|SpawnSystemAttached "/Game/FX/VFX/NS_Slash.NS_Slash" (Variables|Default|GetAttackSpawn) "None" "0, 0, 0" "0, 0, 0" "KeepRelativeOffset" false)
  (bind _outactors (Collision|SphereOverlapActors (Transformation|GetWorldLocation (Variables|Default|GetAttackSpawn)) (Variables|Default|GetRadiusOfAttack) (Variables|Default|GetObjectTypesToAttack) 0))
  (for _array_element _outactors
    (bind _asbp_enemy_base (Utilities|Casting|CastToBP_EnemyBase _array_element))
    (Default|TakeDamage _asbp_enemy_base (Variables|Default|GetDamageToDo) (Variables|Default|GetPoisonEnabled))))
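; Base projectile actor for weapons that damages characters on the opposing side and then destroys itself.
; On overlap, it branches on the owner type: player shots damage enemies and pass a poison flag, while enemy shots damage only the player.
; Overlaps with other actors are ignored, and any blocking hit destroys the projectile.
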(event OnComponentBeginOverlap(Collision)
  (params (OverlappedComponent :type Primitive%20Component%20Object%20Reference) (OtherActor :type Actor%20Object%20Reference) (OtherComp :type Primitive%20Component%20Object%20Reference) (OtherBodyIndex :type Integer) (bFromSweep :type Boolean) (SweepResult :type Hit%20Result%20Structure%20%28by%20ref%29))
  (switch Utilities|FlowControl|Switch|SwitchonE_ProjectileOwner (Variables|Default|GetProjectileOwnerType)
    (:NewEnumerator0
      (bind _asbp_enemy_base (Utilities|Casting|CastToBP_EnemyBase OtherActor))
      (Default|TakeDamage _asbp_enemy_base (Variables|Default|GetDamage) (Variables|Default|GetHasPoison)))
    (:NewEnumerator1
      (bind _asbp_player_base (Utilities|Casting|CastToBP_PlayerBase OtherActor))
      (Default|TakeDamage _asbp_player_base (Variables|Default|GetDamage))))
  (Actor|DestroyActor))

(event OnComponentHit(Collision)
  (params (HitComponent :type Primitive%20Component%20Object%20Reference) (OtherActor :type Actor%20Object%20Reference) (OtherComp :type Primitive%20Component%20Object%20Reference) (NormalImpulse :type Vector :default "0, 0, 0") (Hit :type Hit%20Result%20Structure%20%28by%20ref%29))
  (Actor|DestroyActor))

(fn ConstructionScript)
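; BP_HackZone is a temporary area-of-effect zone that slows and damages enemies inside it.
; On BeginPlay it sets its lifespan and starts a looping timer that applies damage without poison to every valid tracked enemy.
; DamageZone overlap events add or remove BP_EnemyBase actors from EnemiesInside, scaling their walk speed on entry and restoring the default on exit.
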(event OnComponentBeginOverlap(DamageZone)
  (params (OverlappedComponent :type Primitive%20Component%20Object%20Reference) (OtherActor :type Actor%20Object%20Reference) (OtherComp :type Primitive%20Component%20Object%20Reference) (OtherBodyIndex :type Integer) (bFromSweep :type Boolean) (SweepResult :type Hit%20Result%20Structure%20%28by%20ref%29))
  (bind _asbp_enemy_base (Utilities|Casting|CastToBP_EnemyBase OtherActor))
  (Utilities|Array|AddUnique (Variables|Default|GetEnemiesInside) _asbp_enemy_base)
  (Variables|/Script/Engine.CharacterMovementComponent|SetMaxWalkSpeed (Variables|/Script/Engine.Character|GetCharacterMovement _asbp_enemy_base) (* (Variables|/Game/Blueprint/Enemy/BP_EnemyBase.BP_EnemyBase_C|GetDefaultMoveSpeed _asbp_enemy_base) (Variables|Default|GetSlowMultiplier))))

(event OnComponentEndOverlap(DamageZone)
  (params (OverlappedComponent :type Primitive%20Component%20Object%20Reference) (OtherActor :type Actor%20Object%20Reference) (OtherComp :type Primitive%20Component%20Object%20Reference) (OtherBodyIndex :type Integer))
  (bind _asbp_enemy_base (Utilities|Casting|CastToBP_EnemyBase OtherActor))
  (Utilities|Array|RemoveItem (Variables|Default|GetEnemiesInside) _asbp_enemy_base)
  (Variables|/Script/Engine.CharacterMovementComponent|SetMaxWalkSpeed (Variables|/Script/Engine.Character|GetCharacterMovement _asbp_enemy_base) (Variables|/Game/Blueprint/Enemy/BP_EnemyBase.BP_EnemyBase_C|GetDefaultMoveSpeed _asbp_enemy_base)))

(event Custom|ApplyZoneDamage
  (for _array_element (Variables|Default|GetEnemiesInside)
    (Utilities|IsValid _array_element
      (:Is%20Valid
        (Default|TakeDamage _array_element (Variables|Default|GetDamagePerTick) false)))))

(event EventBeginPlay
  (Actor|SetLifeSpan (Variables|Default|GetLifetime))
  (Utilities|Time|SetTimerbyEvent (delegate Custom|ApplyZoneDamage) (Variables|Default|GetTickRate) true))

(fn ConstructionScript)
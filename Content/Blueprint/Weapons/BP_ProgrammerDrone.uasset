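; BP_ProgrammerDrone is a temporary companion drone that follows its owning player and automatically shoots nearby enemies.
; Tick interpolates the drone toward an offset above and to one side of the player's mesh.
; A looping fire-rate timer sphere-overlaps for BP_EnemyBase actors, picks the closest, and spawns a projectile aimed at it, passing along the drone's damage.
; The drone expires after its configured lifetime.
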(event Custom|FireAtNearestEnemy
  (bind _returnvalue (Transformation|GetActorLocation))
  (Variables|Default|SetClosestEnemy 0)
  (Variables|Default|SetClosestDistance 99999.0)
  (bind _outactors (Collision|SphereOverlapActors (Transformation|GetWorldLocation (Variables|Default|GetCube)) 1e+03 (Variables|Default|GetObject%20Types) "/Game/Blueprint/Enemy/BP_EnemyBase.BP_EnemyBase_C"))
  (for _array_element _outactors
    (bind _asbp_enemy_base (Utilities|Casting|CastToBP_EnemyBase _array_element))
    (if (< (Math|Vector|Distance(Vector) (Transformation|GetActorLocation) (Transformation|GetActorLocation _asbp_enemy_base)) (Variables|Default|GetClosestDistance))
      (Variables|Default|SetClosestEnemy _asbp_enemy_base)
      (Variables|Default|SetClosestDistance (Math|Vector|Distance(Vector) (Transformation|GetActorLocation) (Transformation|GetActorLocation _asbp_enemy_base)))))
  (Utilities|IsValid (Variables|Default|GetClosestEnemy)
    (:Is%20Valid
      (Game|SpawnActorfromClass (Variables|Default|GetProjectileClass) (Math|Transform|MakeTransform _returnvalue (Math|Rotator|FindLookatRotation _returnvalue (Transformation|GetActorLocation (Variables|Default|GetClosestEnemy))) "1.000000,1.000000,1.000000") "Undefined" "MultiplyWithRoot" 0 (Variables|Default|GetDamage) "NewEnumerator0" false 0))))

(event EventBeginPlay
  (Actor|SetLifeSpan (Variables|Default|GetLifetime))
  (Utilities|Time|SetTimerbyEvent (delegate Custom|FireAtNearestEnemy) (Variables|Default|GetFireRate) true))

(event EventTick
  (params (DeltaSeconds :type Float%20%28single-precision%29))
  (bind _ownerplayer (Variables|Default|GetOwnerPlayer))
  (bind _mesh (Variables|/Script/Engine.Character|GetMesh _ownerplayer))
  (Utilities|IsValid (Variables|Default|GetOwnerPlayer)
    (:Is%20Valid
      (Transformation|SetActorLocation (Math|Interpolation|VInterpTo (Transformation|GetWorldLocation (Variables|Default|GetCube)) (+ (Transformation|GetWorldLocation _mesh) (* (Math|Vector|GetRightVector _mesh) -1.5e+02) (* (Math|Vector|GetUpVector _mesh) 1e+02)) 0.0 0.0) false false))))

(fn ConstructionScript)